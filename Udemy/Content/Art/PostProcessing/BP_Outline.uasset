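; Demo actor that adjusts a post-process outline radius from keyboard input and scales a sphere to audio loudness.
; While R or F is held, Tick nudges the Radius parameter in MPC_Outline up or down within bounds and prints it.
; Construction copies the LoudnessAnalyzer's sound to the Music component, whose playback-percent event samples normalized loudness to drive the Sphere's scale.
; The Music Play call is unwired, so this graph never starts playback.
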(event Custom|AudioPlaybackPercent
  (params (PlayingSoundWave :type Sound%20Wave%20Object%20Reference) (PlaybackPercent :type Float%20%28single-precision%29))
  (Transformation|SetRelativeScale3D (Variables|Default|GetSphere) (Math|Conversions|ToVector(Float) (+ (* (Class|LoudnessNRT|GetNormalizedLoudnessatTime (Variables|Default|GetLoudnessAnalyzer) (* PlaybackPercent (Variables|Default|GetDuration))) 2.0) 1.0))))

(event EventBeginPlay
  (Input|EnableInput (Game|GetPlayerController 0))
  (EventDispatchers|BindEventtoOnAudioPlaybackPercent (Variables|Default|GetMusic) (delegate Custom|AudioPlaybackPercent)))

(event Collision|EventActorBeginOverlap
  (params (OtherActor :type Actor%20Object%20Reference)))

(event EventTick
  (params (DeltaSeconds :type Float%20%28single-precision%29))
  (Utilities|FlowControl|Sequence
    (:then_0
      (bind _returnvalue (Rendering|Material|GetScalarParameterValue "/Game/Art/PostProcessing/MPC_Outline.MPC_Outline" "Radius" :!class /Script/Engine.KismetMaterialLibrary))
      (if (and (Variables|Default|GetInputIncreasePress) (<= _returnvalue 1.0))
        (Rendering|Material|SetScalarParameterValue "/Game/Art/PostProcessing/MPC_Outline.MPC_Outline" "Radius" (+ _returnvalue 0.01) :!class /Script/Engine.KismetMaterialLibrary)
        (Development|PrintString (Utilities|String|ToString(Float) _returnvalue))))
    (:then_1
      (bind _returnvalue_2 (Rendering|Material|GetScalarParameterValue "/Game/Art/PostProcessing/MPC_Outline.MPC_Outline" "Radius" :!class /Script/Engine.KismetMaterialLibrary))
      (if (and (Variables|Default|GetInputDecreasePress) (>= _returnvalue_2 0.0))
        (Rendering|Material|SetScalarParameterValue "/Game/Art/PostProcessing/MPC_Outline.MPC_Outline" "Radius" (- _returnvalue_2 0.01) :!class /Script/Engine.KismetMaterialLibrary)
        (Development|PrintString (Utilities|String|ToString(Float) _returnvalue_2))))))

(event Input|KeyboardEvents|R
  (params (Key :type Key%20Structure))
  (:Pressed
    (Variables|Default|SetInputIncreasePress true))
  (:Released
    (Variables|Default|SetInputIncreasePress false)))

(event Input|KeyboardEvents|F
  (params (Key :type Key%20Structure))
  (:Pressed
    (Variables|Default|SetInputDecreasePress true))
  (:Released
    (Variables|Default|SetInputDecreasePress false)))

(fn ConstructionScript
  (bind _loudnessanalyzer (Variables|Default|GetLoudnessAnalyzer))
  (bind _sound (Variables|/Script/AudioAnalyzer.AudioAnalyzerNRT|GetSound _loudnessanalyzer))
  (Audio|Components|Audio|SetSound (Variables|Default|GetMusic) _sound)
  (Variables|Default|SetDuration (Variables|/Script/Engine.SoundBase|GetDuration _sound)))