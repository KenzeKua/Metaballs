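; Metaball controller Blueprint that feeds three sphere vectors into the MPC_Metaballs material parameter collection.
; SetActorLocation writes Sphere1 to Sphere3 at BeginPlay, then about every 0.1 seconds through a Delay on Tick when TickEnabled is set.
; Values come from the GetActorLocation helper, whose only node, shown as unused, packs a MetaballsLocation actor's position and roll into a linear color.
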(event EventBeginPlay
  (CallFunction|SetActorLocation)
  (Actor|Tick|SetActorTickEnabled (Variables|Default|GetTickEnabled)))

(event Collision|EventActorBeginOverlap
  (params (OtherActor :type Actor%20Object%20Reference)))

(event EventTick
  (params (DeltaSeconds :type Float%20%28single-precision%29))
  (Utilities|FlowControl|Delay 0.1)
  (CallFunction|SetActorLocation))

(fn ConstructionScript)

(fn SetActorLocation
  (Rendering|Material|SetVectorParameterValue "/Game/Art/Metaballs/MPC_Metaballs.MPC_Metaballs" "Sphere1" (Utilities|GetActorLocation) :!class /Script/Engine.KismetMaterialLibrary)
  (Rendering|Material|SetVectorParameterValue "/Game/Art/Metaballs/MPC_Metaballs.MPC_Metaballs" "Sphere2" (Utilities|GetActorLocation 1) :!class /Script/Engine.KismetMaterialLibrary)
  (Rendering|Material|SetVectorParameterValue "/Game/Art/Metaballs/MPC_Metaballs.MPC_Metaballs" "Sphere3" (Utilities|GetActorLocation 2) :!class /Script/Engine.KismetMaterialLibrary))