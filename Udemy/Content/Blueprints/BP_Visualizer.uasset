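; Interactive music visualizer actor that drives a Niagara particle grid from the song's spectrum.
; Box overlap enables player input and lights an indicator; E starts or pauses the music, with play state shown by indicator colour.
; Playback-percent events sample pre-analysed Constant-Q data at the current time, pushing scaled and normalized arrays into Niagara.
; The static-mesh bar functions are unused.
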(event OnComponentBeginOverlap(BoxCollision)
  (params (OverlappedComponent :type Primitive%20Component%20Object%20Reference) (OtherActor :type Actor%20Object%20Reference) (OtherComp :type Primitive%20Component%20Object%20Reference) (OtherBodyIndex :type Integer) (bFromSweep :type Boolean) (SweepResult :type Hit%20Result%20Structure%20%28by%20ref%29))
  (if (== (Game|GetInstigatorController (Components|GetOwner OtherActor)) (Game|GetInstigatorController (Game|GetPlayerController 0)))
    (Input|EnableInput (Game|GetPlayerController 0))
    (Rendering|Material|SetScalarParameterValue (Variables|Default|GetEnterIndicatorDynamicMat) "Emission" 1.0 :!class /Script/Engine.MaterialInstanceDynamic)))

(event OnComponentEndOverlap(BoxCollision)
  (params (OverlappedComponent :type Primitive%20Component%20Object%20Reference) (OtherActor :type Actor%20Object%20Reference) (OtherComp :type Primitive%20Component%20Object%20Reference) (OtherBodyIndex :type Integer))
  (if (== (Game|GetInstigatorController (Components|GetOwner OtherActor)) (Game|GetInstigatorController (Game|GetPlayerController 0)))
    (Input|DisableInput (Game|GetPlayerController 0))
    (Rendering|Material|SetScalarParameterValue (Variables|Default|GetEnterIndicatorDynamicMat) "Emission" 0.0 :!class /Script/Engine.MaterialInstanceDynamic)))

(event Custom|UpdateSpectrum
  (params (PlayingSoundWave :type Sound%20Wave%20Object%20Reference) (PlaybackPercent :type Float%20%28single-precision%29))
  (CallFunction|UpdateNiagara (* (Variables|/Script/Engine.SoundBase|GetDuration PlayingSoundWave) PlaybackPercent)))

(event EventBeginPlay
  (Audio|Components|Audio|SetSound (Variables|Default|GetMusic) (Variables|/Script/AudioAnalyzer.AudioAnalyzerNRT|GetSound (Variables|Default|GetConstQAnalyzer)))
  (CallFunction|InitializeNiagara)
  (Utilities|FlowControl|Sequence
    (:then_0
      (bind _returnvalue (Rendering|Material|CreateDynamicMaterialInstance (Variables|Default|GetEnterIndicator) 0 "/Game/Niagara/MI_Indicator1.MI_Indicator1" "None" :!class /Script/Engine.PrimitiveComponent))
      (bind _output_get (Variables|Default|SetEnterIndicatorDynamicMat _returnvalue))
      (Rendering|Material|SetScalarParameterValue _output_get "Emission" 0.0 :!class /Script/Engine.MaterialInstanceDynamic)
      (Rendering|Material|SetVectorParameterValue _output_get "Colour" "(R=0.102059,G=0.493480,B=0.859375,A=1.000000)" :!class /Script/Engine.MaterialInstanceDynamic))
    (:then_1
      (bind _returnvalue_2 (Rendering|Material|CreateDynamicMaterialInstance (Variables|Default|GetPlayIndicator) 0 "/Game/Niagara/MI_Indicator1.MI_Indicator1" "None" :!class /Script/Engine.PrimitiveComponent))
      (bind _output_get_2 (Variables|Default|SetPlayIndicatorDynamicMat _returnvalue_2))
      (Rendering|Material|SetScalarParameterValue _output_get_2 "Emission" 0.7 :!class /Script/Engine.MaterialInstanceDynamic)
      (Rendering|Material|SetVectorParameterValue _output_get_2 "Colour" "(R=1.000000,G=0.000000,B=0.024691,A=1.000000)" :!class /Script/Engine.MaterialInstanceDynamic))))

(event Collision|EventActorBeginOverlap
  (params (OtherActor :type Actor%20Object%20Reference)))

(event EventTick
  (params (DeltaSeconds :type Float%20%28single-precision%29)))

(event Input|KeyboardEvents|E
  (params (Key :type Key%20Structure))
  (bind _playindicatordynamicmat (Variables|Default|GetPlayIndicatorDynamicMat))
  (bind _music (Variables|Default|GetMusic))
  (:Pressed
    (if (Audio|Components|Audio|IsPlaying _music)
      (Utilities|FlowControl|FlipFlop
        (:A
          (Class|AudioComponent|SetPaused _music true)
          (Rendering|Material|SetVectorParameterValue _playindicatordynamicmat "Colour" "(R=1.000000,G=0.000000,B=0.024691,A=1.000000)" :!class /Script/Engine.MaterialInstanceDynamic))
        (:B
          (Class|AudioComponent|SetPaused _music false)
          (Rendering|Material|SetVectorParameterValue _playindicatordynamicmat "Colour" "(R=0.083878,G=0.864583,B=0.000000,A=1.000000)" :!class /Script/Engine.MaterialInstanceDynamic :!label _label)))
      (else
        (EventDispatchers|BindEventtoOnAudioPlaybackPercent _music (delegate Custom|UpdateSpectrum))
        (if (Variables|Default|GetPlaySong)
          (Audio|Components|Audio|Play _music 0.0)
          (goto _label))))))

(fn ConstructionScript)

(fn ConstructStaticMesh
  (bind _barcount (Variables|Default|GetBarCount))
  (bind _barspacing (Variables|Default|GetBarSpacing))
  (bind _barspacing_2 (Variables|Default|GetBarSpacing))
  (bind (_x _y) (Utilities|Struct|BreakIntVector _barcount))
  (bind _returnvalue (- _x 1))
  (bind _returnvalue_2 (- _y 1))
  (for _index (range 0 _returnvalue)
    (for _index_2 (range 0 _returnvalue_2)
      (bind _returnvalue_3 (AddComponent|AddStaticMeshComponent false (Math|Transform|MakeTransform (Math|Vector|MakeVector (- (* _index _barspacing_2) (/ (* _returnvalue _barspacing_2) 2.0)) (- (* _index_2 _barspacing) (/ (* _returnvalue_2 _barspacing) 2.0)) 0.0))))
      (Components|StaticMesh|SetStaticMesh _returnvalue_3 (Variables|Default|GetBarShape))
      (Utilities|Array|Add (Variables|Default|GetBarsArray) _returnvalue_3))))

(fn UpdateStaticMesh
  (params (PlaybackPercent :type Float%20%28single-precision%29))
  (for (_array_element _array_index) (Class|ConstantQNRT|GetNormalizedChannelConstantQatTime (Variables|Default|GetConstQAnalyzer) PlaybackPercent)
    (Transformation|SetRelativeScale3D (Utilities|Array|Get(acopy) (Variables|Default|GetBarsArray) _array_index) (Math|Vector|MakeVector 1.0 1.0 (.z (Math|Interpolation|VInterpTo (Math|Vector|MakeVector 0.0 0.0 (.z (Variables|/Script/Engine.SceneComponent|GetRelativeScale3D (Utilities|Array|Get(acopy) (Variables|Default|GetBarsArray) _array_index)))) (Math|Vector|MakeVector 0.0 0.0 (+ (* _array_element 7.0) 1.0)) (Utilities|Time|GetWorldDeltaSeconds) 5e+01))))))

(fn InitializeNiagara
  (bind _niagaravisualizer (Variables|Default|GetNiagaraVisualizer))
  (bind _barcount (Variables|Default|GetBarCount))
  (bind _returnvalue (Math|Conversions|ToVector(Float) _barcount))
  (bind (_x _y _z) (Math|Vector|BreakVector _returnvalue))
  (Effects|Components|ParticleSystem|SetFloatParameter _niagaravisualizer "User.XParticleCount" _x)
  (Effects|Components|ParticleSystem|SetFloatParameter _niagaravisualizer "User.YParticleCount" _y)
  (Effects|Components|ParticleSystem|SetFloatParameter _niagaravisualizer "User.ZParticleCount" _z)
  (Effects|Components|ParticleSystem|SetFloatParameter _niagaravisualizer "User.ParticleStepSize" (Variables|Default|GetBarSpacing)))

(fn UpdateNiagara
  (params (PlaybackDuration :type Float%20%28single-precision%29))
  (bind _constqanalyzer (Variables|Default|GetConstQAnalyzer))
  (bind _niagaravisualizer (Variables|Default|GetNiagaraVisualizer))
  (bind _outconstantq (Class|ConstantQNRT|GetNormalizedChannelConstantQatTime _constqanalyzer PlaybackDuration))
  (bind _output_get (Variables|Default|SetNiagaraOutSpectrum _outconstantq))
  (CallFunction|CalculateScaleNiagara)
  (Class|NiagaraDataInterfaceArrayFunctionLibrary|SetNiagaraArrayFloat _niagaravisualizer "User.OutSpectrum" _output_get)
  (Class|NiagaraDataInterfaceArrayFunctionLibrary|SetNiagaraArrayFloat _niagaravisualizer "User.NormalizedSpectrum" _outconstantq))

(fn CalculateScaleNiagara
  (for (_array_element _array_index) (Variables|Default|GetNiagaraOutSpectrum)
    (Utilities|Array|SetArrayElem (Variables|Default|GetNiagaraOutSpectrum) _array_index (* (+ _array_element 0.0) 13.0))))